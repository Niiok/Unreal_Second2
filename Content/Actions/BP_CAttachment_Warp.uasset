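; BP_CAttachment_Warp is an attachment Blueprint, named for a Warp action, that controls the visibility of a Decal while it is equipped.
; The Decal is hidden on BeginPlay, shown on OnEquip and hidden again on OnUnequip, each after calling the parent event.
; It holds no warp or decal placement logic, and its Tick and overlap events are empty.
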(event Collision|EventActorBeginOverlap
  (params (OtherActor :type Actor%20Object%20Reference)))

(event EventTick
  (params (DeltaSeconds :type Float%20%28single-precision%29)))

(event EventBeginPlay
  (|CallParentFunction)
  (Rendering|SetVisibility (Variables|Default|GetDecal) false false))

(event EventOnEquip
  (|CallParentFunction)
  (Rendering|SetVisibility (Variables|Default|GetDecal) true false))

(event EventOnUnequip
  (|CallParentFunction)
  (Rendering|SetVisibility (Variables|Default|GetDecal) false false))

(fn ConstructionScript)